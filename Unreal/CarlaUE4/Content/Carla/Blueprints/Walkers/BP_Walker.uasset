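; CARLA pedestrian walker that can carry a prop and ragdolls when struck by a vehicle.
; Prop attaches a collisionless static mesh to a socket and sizes a second death trigger around it.
; Unless invincible, either trigger overlapping a vehicle's skeletal mesh drops the prop, enables body physics, shrinks the collision volumes and destroys the actor after AfterLifeSpan.
; Foot IK trace and trolley-angle helpers remain, but the trolley logic is disconnected.
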(event OnComponentBeginOverlap(PedestrianDeathTrigger)
  (params (OverlappedComponent :type Primitive%20Component%20Object%20Reference) (OtherActor :type Actor%20Object%20Reference) (OtherComp :type Primitive%20Component%20Object%20Reference) (OtherBodyIndex :type Integer) (bFromSweep :type Boolean) (SweepResult :type Hit%20Result%20Structure%20%28by%20ref%29))
  (if (not (Variables|Default|GetbIsInvincible))
    (Utilities|HitbySomething OtherActor OtherComp)))

(event OnComponentBeginOverlap(PedestrianPropDeathTrigger)
  (params (OverlappedComponent :type Primitive%20Component%20Object%20Reference) (OtherActor :type Actor%20Object%20Reference) (OtherComp :type Primitive%20Component%20Object%20Reference) (OtherBodyIndex :type Integer) (bFromSweep :type Boolean) (SweepResult :type Hit%20Result%20Structure%20%28by%20ref%29))
  (if (not (Variables|Default|GetbIsInvincible))
    (Utilities|HitbySomething OtherActor OtherComp)))

(event Collision|EventActorBeginOverlap
  (params (OtherActor :type Actor%20Object%20Reference)))

(event EventTick
  (params (DeltaSeconds :type Float%20%28single-precision%29))
  ;[1 1 1] DebugLine__CarlaWorks
)

(fn ConstructionScript)

(fn Prop
  (params (Prop%20to%20place :type Static%20Mesh%20Object%20Reference) (SocketName :type Name) (RelativeTransform :type Transform))
  (bind _returnvalue (StaticMesh|GetBoundingBox Prop%20to%20place))
  (bind _pedestrianpropdeathtrigger (Variables|Components|GetPedestrianPropDeathTrigger))
  (bind _returnvalue_2 (- (.z (.max _returnvalue)) (.z (.min _returnvalue))))
  (bind _returnvalue_3 (/ _returnvalue_2 2.0))
  (Variables|Default|SetHoldsProp true)
  (Utilities|FlowControl|Sequence
    (:then_0
      ;[1 1 1] Add Component
      (bind _returnvalue_4 (AddComponent|AddStaticMeshComponent false RelativeTransform))
      (Variables|Components|SetHoldMesh _returnvalue_4)
      (Components|StaticMesh|SetStaticMesh (Variables|Components|GetHoldMesh) Prop%20to%20place)
      (Transformation|AttachComponentToComponent (Variables|Components|GetHoldMesh) (Variables|Character|GetMesh) SocketName "KeepRelative" "KeepRelative" "KeepRelative" true)
      (Collision|SetCollisionEnabled (Variables|Components|GetHoldMesh) "NoCollision")
      (bind _ascarla_game_instance (Utilities|Casting|CastToCarlaGameInstance (Game|GetGameInstance)))
      (Class|CarlaGameInstance|GetCARLASettings _ascarla_game_instance)
      (Class|PrimitiveComponent|SetCullDistance (Variables|Components|GetHoldMesh) 0.0))
    (:then_1
      ;[1 1 1] Extend Carcrash box
      (Transformation|AttachComponentToComponent _pedestrianpropdeathtrigger (Variables|Components|GetHoldMesh) "None" "KeepRelative" "KeepRelative" "KeepRelative" true)
      (Components|Box|SetBoxExtent _pedestrianpropdeathtrigger (Math|Vector|MakeVector (+ (/ (- (.x (.max _returnvalue)) (.x (.min _returnvalue))) 2.0) 1e+01) (+ (/ (- (.y (.max _returnvalue)) (.y (.min _returnvalue))) 2.0) 1e+01) (+ _returnvalue_3 1e+01)) true)
      (Transformation|SetRelativeTransform _pedestrianpropdeathtrigger (Math|Transform|MakeTransform (Math|Vector|MakeVector 0.0 0.0 (- 1.0 _returnvalue_3)) "0, 0, 0" "1,1,1") true false))
    (:then_2)
    (:then_3
      (return (Variables|Character|GetMesh) Prop%20to%20place (Variables|Components|GetHoldMesh)))))

(fn HitbyCar
  (bind _mesh (Variables|Character|GetMesh))
  (bind _holdmesh (Variables|Components|GetHoldMesh))
  (if (Utilities|IsValid _holdmesh)
    (Transformation|DetachFromComponent _holdmesh "KeepWorld" "KeepWorld" "KeepWorld" true)
    (Physics|SetSimulatePhysics _holdmesh true)
    (Collision|SetCollisionEnabled _holdmesh "QueryAndPhysics"))
  (Physics|SetSimulatePhysics _mesh true)
  (Collision|SetCollisionEnabled _mesh "QueryAndPhysics")
  (Components|Box|SetBoxExtent (Variables|Components|GetPedestrianDeathTrigger) "1.000000,1.000000,1.000000" true)
  (Components|Box|SetBoxExtent (Variables|Components|GetPedestrianPropDeathTrigger) "1.000000,1.000000,1.000000" true)
  (Components|Box|SetBoxExtent (Variables|Components|GetCarStopper) "20.000000,20.000000,20.000000" true)
  (Components|Capsule|SetCapsuleSize (Variables|Collision|GetCapsuleComponent) 0.0 0.0 true)
  (Collision|SetCollisionResponsetoAllChannels (Variables|Character|GetMesh) "ECR_Block"))

(fn IKFootTrace
  (params (InSocketName :type Name) (TraceDistance :type Float%20%28single-precision%29))
  (bind _returnvalue (Transformation|GetActorLocation))
  (bind _mesh (Variables|Character|GetMesh))
  (bind _returnvalue_2 (Transformation|GetSocketLocation _mesh InSocketName))
  (bind _z (Math|Vector|BreakVector _returnvalue))
  (bind (_x _y) (Math|Vector|BreakVector _returnvalue_2))
  (bind _returnvalue_3 (- _z TraceDistance))
  (bind _returnvalue_4 (Math|Vector|MakeVector _x _y _returnvalue_3))
  (bind (_outhit _returnvalue_5) (Collision|LineTraceByChannel (Math|Vector|MakeVector _x _y _z) _returnvalue_4 "TraceTypeQuery1" true 0 "Persistent"))
  (return (Math|Float|SelectFloat (/ (Math|Vector|VectorLength (- _returnvalue_4 (.Location (Collision|BreakHitResult _outhit)))) (Variables|IkDataSetup|GetIkScale)) 0.0 _returnvalue_5)))
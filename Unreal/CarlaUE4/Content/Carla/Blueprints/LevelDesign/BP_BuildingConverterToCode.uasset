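; Level design utility that migrates Blueprint procedural buildings to the native C++ ProceduralBuilding class.
; Convert finds every BP_Procedural_Bulding in the level and spawns a native building at the same transform.
; It passes the old actor to a native conversion call, then copies dimensions, visibility and mesh/Blueprint sets for base, body, top and roof.
; Each original actor is destroyed afterward; construction and event graphs are empty.
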(event EventBeginPlay)

(event Collision|EventActorBeginOverlap
  (params (OtherActor :type Actor%20Object%20Reference)))

(event EventTick
  (params (DeltaSeconds :type Float%20%28single-precision%29)))

(fn ConstructionScript)

(fn Convert
  (bind _outactors (Actor|GetAllActorsOfClass "/Game/Carla/Blueprints/LevelDesign/BP_Procedural_Bulding.BP_Procedural_Bulding_C"))
  (for _array_element _outactors
    (LocalVariables|SetBP_Building _array_element)
    (Utilities|FlowControl|Sequence
      (:then_0
        ;[1 1 1] Create the new building
        (bind _returnvalue (Game|SpawnActorfromClass "/Script/Carla.ProceduralBuilding" (Transformation|GetActorTransform (LocalVariables|GetBP_Building)) "AlwaysSpawn" 0 0))
        (bind _output_get (LocalVariables|SetNewProceduralBuilding _returnvalue))
        (Class|ProceduralBuilding|ConvertOldBPtoNativeCodeObject _output_get (LocalVariables|GetBP_Building)))
      (:then_1
        (Class|ProceduralBuilding|SetBaseParameters (LocalVariables|GetNewProceduralBuilding) (Variables|/Game/Carla/Blueprints/LevelDesign/BP_Procedural_Bulding.BP_Procedural_Bulding_C|GetDoors (LocalVariables|GetBP_Building)) (Variables|/Game/Carla/Blueprints/LevelDesign/BP_Procedural_Bulding.BP_Procedural_Bulding_C|GetWalls (LocalVariables|GetBP_Building)) (Variables|/Game/Carla/Blueprints/LevelDesign/BP_Procedural_Bulding.BP_Procedural_Bulding_C|GetNumFloors (LocalVariables|GetBP_Building)) (Variables|/Game/Carla/Blueprints/LevelDesign/BP_Procedural_Bulding.BP_Procedural_Bulding_C|GetLengthX (LocalVariables|GetBP_Building)) (Variables|/Game/Carla/Blueprints/LevelDesign/BP_Procedural_Bulding.BP_Procedural_Bulding_C|GetLengthY (LocalVariables|GetBP_Building)) (Variables|/Game/Carla/Blueprints/LevelDesign/BP_Procedural_Bulding.BP_Procedural_Bulding_C|GetCorners (LocalVariables|GetBP_Building)) (Variables|/Game/Carla/Blueprints/LevelDesign/BP_Procedural_Bulding.BP_Procedural_Bulding_C|GetUseFullBlocks (LocalVariables|GetBP_Building)))
        (Class|ProceduralBuilding|SetVisibilityParameters (LocalVariables|GetNewProceduralBuilding) (Variables|/Game/Carla/Blueprints/LevelDesign/BP_Procedural_Bulding.BP_Procedural_Bulding_C|GetSideVisibility (LocalVariables|GetBP_Building)) (Variables|/Game/Carla/Blueprints/LevelDesign/BP_Procedural_Bulding.BP_Procedural_Bulding_C|GetCornerVisibility (LocalVariables|GetBP_Building)) (Variables|/Game/Carla/Blueprints/LevelDesign/BP_Procedural_Bulding.BP_Procedural_Bulding_C|GetRoofVisibility (LocalVariables|GetBP_Building)))
        (Class|ProceduralBuilding|SetBaseMeshes (LocalVariables|GetNewProceduralBuilding) (Variables|/Game/Carla/Blueprints/LevelDesign/BP_Procedural_Bulding.BP_Procedural_Bulding_C|GetBaseMeshes (LocalVariables|GetBP_Building)) (Variables|/Game/Carla/Blueprints/LevelDesign/BP_Procedural_Bulding.BP_Procedural_Bulding_C|GetBaseBPs (LocalVariables|GetBP_Building)) (Variables|/Game/Carla/Blueprints/LevelDesign/BP_Procedural_Bulding.BP_Procedural_Bulding_C|GetCornerBaseMeshes (LocalVariables|GetBP_Building)) (Variables|/Game/Carla/Blueprints/LevelDesign/BP_Procedural_Bulding.BP_Procedural_Bulding_C|GetCornerBaseBPs (LocalVariables|GetBP_Building)) (Variables|/Game/Carla/Blueprints/LevelDesign/BP_Procedural_Bulding.BP_Procedural_Bulding_C|GetDoorMeshes (LocalVariables|GetBP_Building)) (Variables|/Game/Carla/Blueprints/LevelDesign/BP_Procedural_Bulding.BP_Procedural_Bulding_C|GetDoorBPs (LocalVariables|GetBP_Building)))
        (Class|ProceduralBuilding|SetBodyMeshes (LocalVariables|GetNewProceduralBuilding) (Variables|/Game/Carla/Blueprints/LevelDesign/BP_Procedural_Bulding.BP_Procedural_Bulding_C|GetBodyMeshes (LocalVariables|GetBP_Building)) (Variables|/Game/Carla/Blueprints/LevelDesign/BP_Procedural_Bulding.BP_Procedural_Bulding_C|GetBodyBPs (LocalVariables|GetBP_Building)) (Variables|/Game/Carla/Blueprints/LevelDesign/BP_Procedural_Bulding.BP_Procedural_Bulding_C|GetCornerBodyMeshes (LocalVariables|GetBP_Building)) (Variables|/Game/Carla/Blueprints/LevelDesign/BP_Procedural_Bulding.BP_Procedural_Bulding_C|GetCornerBodyBPs (LocalVariables|GetBP_Building)) (Variables|/Game/Carla/Blueprints/LevelDesign/BP_Procedural_Bulding.BP_Procedural_Bulding_C|GetWallMeshes (LocalVariables|GetBP_Building)) (Variables|/Game/Carla/Blueprints/LevelDesign/BP_Procedural_Bulding.BP_Procedural_Bulding_C|GetWallBPs (LocalVariables|GetBP_Building)))
        (Class|ProceduralBuilding|SetTopMeshes (LocalVariables|GetNewProceduralBuilding) (Variables|/Game/Carla/Blueprints/LevelDesign/BP_Procedural_Bulding.BP_Procedural_Bulding_C|GetTopMeshes (LocalVariables|GetBP_Building)) (Variables|/Game/Carla/Blueprints/LevelDesign/BP_Procedural_Bulding.BP_Procedural_Bulding_C|GetTopBPs (LocalVariables|GetBP_Building)) (Variables|/Game/Carla/Blueprints/LevelDesign/BP_Procedural_Bulding.BP_Procedural_Bulding_C|GetCornerTopMeshes (LocalVariables|GetBP_Building)) (Variables|/Game/Carla/Blueprints/LevelDesign/BP_Procedural_Bulding.BP_Procedural_Bulding_C|GetCornerTopBPs (LocalVariables|GetBP_Building)) (Utilities|Array|MakeArray (Variables|/Game/Carla/Blueprints/LevelDesign/BP_Procedural_Bulding.BP_Procedural_Bulding_C|GetRoofMesh (LocalVariables|GetBP_Building))) (Utilities|Array|MakeArray (Variables|/Game/Carla/Blueprints/LevelDesign/BP_Procedural_Bulding.BP_Procedural_Bulding_C|GetRoofBP (LocalVariables|GetBP_Building)))))
      (:then_2
        ;[1 1 1] Destroy old building
        (Actor|DestroyActor (LocalVariables|GetBP_Building))))))